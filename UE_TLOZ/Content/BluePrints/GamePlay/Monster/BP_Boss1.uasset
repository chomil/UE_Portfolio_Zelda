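; BP_Boss1 is a boss monster that wields a weapon, can be stunned and dissolves on death.
; BeginPlay attaches the weapon to the Weapon_R socket, and any overlap on its eye collision triggers Stunned.
; While HP is depleted, Tick runs DissolveMonster, which lazily creates an M_Dissolve dynamic instance as the mesh's overlay material, then drives its DissolveTime from scaled DeathTime.
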(event OnComponentBeginOverlap(EyeCollision)
  (params (OverlappedComponent :type Primitive%20Component%20Object%20Reference) (OtherActor :type Actor%20Object%20Reference) (OtherComp :type Primitive%20Component%20Object%20Reference) (OtherBodyIndex :type Integer) (bFromSweep :type Boolean) (SweepResult :type Hit%20Result%20Structure%20%28by%20ref%29))
  (Class|Monster|Stunned true))

(event EventBeginPlay
  (bind _weapon (Variables|Default|GetWeapon))
  (Variables|Default|SetWeaponComponent _weapon)
  (Transformation|AttachComponentToComponent _weapon (Variables|Character|GetMesh) "Weapon_R" "KeepRelative" "KeepRelative" "KeepWorld" true))

(event Collision|EventActorBeginOverlap
  (params (OtherActor :type Actor%20Object%20Reference)))

(event EventTick
  (params (DeltaSeconds :type Float%20%28single-precision%29))
  (|DissolveMonster (<= (Variables|Default|GetHP) 0.0)))

(fn ConstructionScript)