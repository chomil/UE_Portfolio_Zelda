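; BP_Arrow is an arrow projectile that damages monsters it overlaps.
; When the arrow mesh overlaps an actor, an arrow tagged PlayerAttack deals fixed damage to a target tagged Monster that casts to Monster, then destroys itself.
; A projectile bounce or stop deactivates movement and turns on mesh physics, but only a bounce also deactivates the Niagara effect.
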(event OnProjectileStop(Movement)
  (params (ImpactResult :type Hit%20Result%20Structure%20%28by%20ref%29))
  (Components|Activation|Deactivate (Variables|Default|GetMovement))
  (Physics|SetSimulatePhysics (Variables|Default|GetArrowMesh) true))

(event OnComponentBeginOverlap(ArrowMesh)
  (params (OverlappedComponent :type Primitive%20Component%20Object%20Reference) (OtherActor :type Actor%20Object%20Reference) (OtherComp :type Primitive%20Component%20Object%20Reference) (OtherBodyIndex :type Integer) (bFromSweep :type Boolean) (SweepResult :type Hit%20Result%20Structure%20%28by%20ref%29))
  (if (Actor|ActorHasTag self "PlayerAttack")
    (if (Actor|ActorHasTag OtherActor "Monster")
      (bind _asmonster (Utilities|Casting|CastToMonster OtherActor))
      (Class|Monster|Damaged _asmonster 1.0)
      (Actor|DestroyActor))))

(event OnProjectileBounce(Movement)
  (params (ImpactResult :type Hit%20Result%20Structure%20%28by%20ref%29) (ImpactVelocity :type Vector%20%28by%20ref%29 :default "0, 0, 0"))
  (Components|Activation|Deactivate (Variables|Default|GetNiagara))
  (Components|Activation|Deactivate (Variables|Default|GetMovement))
  (Physics|SetSimulatePhysics (Variables|Default|GetArrowMesh) true))

(event EventBeginPlay)

(event Collision|EventActorBeginOverlap
  (params (OtherActor :type Actor%20Object%20Reference)))

(event EventTick
  (params (DeltaSeconds :type Float%20%28single-precision%29)))

(fn ConstructionScript)