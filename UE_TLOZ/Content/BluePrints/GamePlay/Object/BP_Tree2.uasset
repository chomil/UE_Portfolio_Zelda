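; BP_Tree2 is a destructible tree actor that starts with 3 HP and loses one each time something begins overlapping its Tree component.
; The Damaged function detects the hit that first brings HP to zero or below, so felling triggers only once.
; Felling swaps the mesh to a stump, spawns a BP_Trunk at the actor transform and spawns BP_Leaf actors at four leaf component transforms.
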(event OnComponentBeginOverlap(Tree)
  (params (OverlappedComponent :type Primitive%20Component%20Object%20Reference) (OtherActor :type Actor%20Object%20Reference) (OtherComp :type Primitive%20Component%20Object%20Reference) (OtherBodyIndex :type Integer) (bFromSweep :type Boolean) (SweepResult :type Hit%20Result%20Structure%20%28by%20ref%29))
  (CallFunction|Damaged 1))

(event EventBeginPlay
  (Variables|Default|SetHP 3))

(event Collision|EventActorBeginOverlap
  (params (OtherActor :type Actor%20Object%20Reference)))

(event EventTick
  (params (DeltaSeconds :type Float%20%28single-precision%29)))

(fn ConstructionScript)

(fn Damaged
  (params (Damage :type Integer))
  (bind _output_get (Variables|Default|SetHP (- (Variables|Default|GetHP) Damage)))
  (if (<= _output_get 0)
    (if (> (+ _output_get Damage) 0)
      (Components|StaticMesh|SetStaticMesh (Variables|Default|GetTree) "/Game/Resources/Tree/Tree2_stump.Tree2_stump")
      (Game|SpawnActorfromClass "/Game/BluePrints/GamePlay/Object/BP_Trunk.BP_Trunk_C" (Transformation|GetActorTransform self) "Undefined" 0 0)
      (|SpawnLeaf_2))))