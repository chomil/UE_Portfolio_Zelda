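; BP_Item is a world item pickup that adds itself to the player's inventory on touch.
; On BeginPlay it looks up item data by SpawnItemName through GlobalGameInstance and applies the DropMesh to its static mesh.
; When an actor tagged Player overlaps ItemCollision, it adds one unequipped item to the inventory held by GlobalGameInstance, then destroys itself.
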(event OnComponentBeginOverlap(ItemCollision)
  (params (OverlappedComponent :type Primitive%20Component%20Object%20Reference) (OtherActor :type Actor%20Object%20Reference) (OtherComp :type Primitive%20Component%20Object%20Reference) (OtherBodyIndex :type Integer) (bFromSweep :type Boolean) (SweepResult :type Hit%20Result%20Structure%20%28by%20ref%29))
  (if (Actor|ActorHasTag OtherActor "Player")
    (bind _asglobal_game_instance (Utilities|Casting|CastToGlobalGameInstance (Game|GetGameInstance)))
    (bind _returnvalue (Class|GlobalGameInstance|GetInventory _asglobal_game_instance))
    (Class|Inventory|AddItem _returnvalue (Variables|Default|GetSpawnItemName) 1 false)
    (Actor|DestroyActor)))

(event EventBeginPlay
  (bind _asglobal_game_instance (Utilities|Casting|CastToGlobalGameInstance (Game|GetGameInstance)))
  (bind _returnvalue (Class|GlobalGameInstance|GetItemDataRef _asglobal_game_instance (Variables|Default|GetSpawnItemName)))
  (bind _output_get (Variables|Default|SetData _returnvalue))
  (Components|StaticMesh|SetStaticMesh (Variables|Default|GetStaticMesh) (.DropMesh (Utilities|Struct|BreakItemData _output_get))))

(event Collision|EventActorBeginOverlap
  (params (OtherActor :type Actor%20Object%20Reference)))

(event EventTick
  (params (DeltaSeconds :type Float%20%28single-precision%29)))

(fn ConstructionScript)