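; BP_Trunk is a trunk object that supports time rewind and displays a progress indicator while rewinding.
; An overlap on the Trunk component turns rewind on and prints a debug message.
; Each tick toggles the widget component's widget visibility with the rewind state and feeds the current-to-max record ratio into WBP_TimeRewind.
; Recording and playback logic are not in these graphs.
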(event OnComponentBeginOverlap(Trunk)
  (params (OverlappedComponent :type Primitive%20Component%20Object%20Reference) (OtherActor :type Actor%20Object%20Reference) (OtherComp :type Primitive%20Component%20Object%20Reference) (OtherBodyIndex :type Integer) (bFromSweep :type Boolean) (SweepResult :type Hit%20Result%20Structure%20%28by%20ref%29))
  (Development|PrintString "Rewind")
  (Class|MovableActor|SetTimeRewind true))

(event EventBeginPlay)

(event Collision|EventActorBeginOverlap
  (params (OtherActor :type Actor%20Object%20Reference)))

(event EventTick
  (params (DeltaSeconds :type Float%20%28single-precision%29))
  (bind _widget (Variables|Default|GetWidget))
  (bind _returnvalue (UserInterface|GetWidget _widget))
  (if (Variables|Default|GetbTimeRewind)
    (Variables|/Script/UMG.Widget|SetVisibility _returnvalue "Visible")
    (bind _aswbp_time_rewind (Utilities|Casting|CastToWBP_TimeRewind _returnvalue))
    (Default|UpdatePercent _aswbp_time_rewind (/ (Math|Conversions|ToFloat(Integer) (Variables|Default|GetCurRecord)) (Math|Conversions|ToFloat(Integer) (Variables|Default|GetMaxRecord))))
    (else
      (Variables|/Script/UMG.Widget|SetVisibility _returnvalue "Hidden"))))

(fn ConstructionScript)