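; Gameplay game mode Blueprint that applies graphics settings and starts the field music when play begins.
; BeginPlay calls QualitySetting, then plays the Hyrule Field day BGM as a 2D sound.
; QualitySetting runs fixed console commands that set the texture streaming pool size and scalability levels for view distance, anti-aliasing, shadows, post-processing, textures, effects, foliage and shading.
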(event EventBeginPlay
  (CallFunction|QualitySetting)
  (Audio|PlaySound2D "/Game/Resources/Sound/BGM/BGM_Hyrule_Field_Day.BGM_Hyrule_Field_Day" 1.0 1.0 0.0 0 0))

(event EventTick
  (params (DeltaSeconds :type Float%20%28single-precision%29)))

(fn ConstructionScript)

(fn QualitySetting
  (Development|ExecuteConsoleCommand "r.Streaming.PoolSize 2000" 0)
  (Development|ExecuteConsoleCommand "sg.ViewDistanceQuality 1" 0)
  (Development|ExecuteConsoleCommand "sg.AntiAliasingQuality 2" 0)
  (Development|ExecuteConsoleCommand "sg.ShadowQuality 2" 0)
  (Development|ExecuteConsoleCommand "sg.PostProcessQuality 2" 0)
  (Development|ExecuteConsoleCommand "sg.TextureQuality 2" 0)
  (Development|ExecuteConsoleCommand "sg.EffectsQuality 2" 0)
  (Development|ExecuteConsoleCommand "sg.FoliageQuality 2" 0)
  (Development|ExecuteConsoleCommand "sg.ShadingQuality 2" 0))